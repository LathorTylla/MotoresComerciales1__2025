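; Projectile actor that flies straight ahead and bursts into fire when it hits a tagged collider.
; On BeginPlay it sets its projectile movement velocity along its forward vector at a fixed speed.
; On overlap with an actor tagged ColliderProjectile, it spawns a smoky fire Niagara effect and a fire sound at its location, then destroys itself.
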(event EventBeginPlay
  (Variables|/Script/Engine.MovementComponent|SetVelocity (Variables|Default|GetProjectileMovement) (* (Transformation|GetActorForwardVector) 500)))

(event Collision|EventActorBeginOverlap
  (params (OtherActor :type Actor%20Object%20Reference))
  (if (Actor|ActorHasTag OtherActor "ColliderProjectile")
    (Niagara|SpawnSystematLocation "/Game/Vefects/Free_Fire/Shared/Particles/NS_Fire_Medium_Smoke.NS_Fire_Medium_Smoke" (Transformation|GetActorLocation))
    (Audio|SpawnSoundatLocation "/Game/Vefects/Free_Fire/Shared/Audio/SFX_FireMedium_L.SFX_FireMedium_L" (Transformation|GetActorLocation) "0, 0, 0" 1.0 1.0 0.0 0 0)
    (Actor|DestroyActor)))

(event EventTick
  (params (DeltaSeconds :type Float%20%28single-precision%29)))

(fn ConstructionScript)